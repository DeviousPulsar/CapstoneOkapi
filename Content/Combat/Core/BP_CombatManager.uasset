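; Combat manager that runs turn-based fights, alternating between a player menu phase and a timed enemy attack.
; BeginPlay assigns controllers, creates the menu and health bar widgets, and locks player movement with UI-only input.
; Finishing a menu selection restores game input and movement, then a timer set to the enemy attack's returned duration resets the turn.
; Tick polls both health values to refresh the bars, though its cached previous values are only reassigned to themselves.
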(event `self.ReceiveTick`
  (params (DeltaSeconds :type "Float (single-precision)"))
  (bind _prevhealth_player (`self.PrevHealth Player`))
  (bind _prevhealth_enemy (`self.PrevHealth Enemy`))
  ; Main Loop
  ;; Init Step
  (if (`self.IsFirstTick`)
    (set `self.IsFirstTick` false)
    (`self.Change Player Health`)
    (`/Game/Combat/Player/Menu.SetCombatManager` (`self.Menu`) self)
    (`/Game/Combat/Player/HealthBarDisplay.SetCombatManager` (`self.healthBars`) self)
    (bind _returnvalue (`CombatPlayer.GetHealth` (`self.PlayerC`)))
    (set `self.PrevHealth Player` _returnvalue)
    (else
      ;; Update Player Healthbar
      (bind _returnvalue_2 (`CombatPlayer.GetHealth` (`self.PlayerC`)))
      (if (!= _returnvalue_2 _prevhealth_player)
        (`self.Change Player Health`)
        (set `self.PrevHealth Player` _prevhealth_player))
      ;; Update Enemy Healthbar
      (bind _returnvalue_3 (`EnemyController.GetHealth` (`self.EnemyC`)))
      (if (!= _returnvalue_3 _prevhealth_enemy)
        (`self.Change Enemy Health`)
        (set `self.PrevHealth Enemy` _prevhealth_enemy)))))

(event `self.ReceiveBeginPlay`
  (bind _healthbars (`self.healthBars`))
  ; Need to ensure controllers actually exist
  (`self.AssignControllers`)
  ; Builds the menu and forces the player to focus on it
  (bind _returnvalue (`|CreateWidget` "/Game/Combat/Player/Menu.Menu_C"))
  (bind _output_get (set `self.Menu` _returnvalue))
  (add `/Game/Combat/Player/Menu.PlayerSelectionFinished` _output_get (delegate `Give Control to Enemy`))
  (`UserWidget.AddToViewport` _output_get 0)
  (`WidgetBlueprintLibrary.SetInputMode_UIOnlyEx` (`GameplayStatics.GetPlayerController` 0) _output_get)
  (`/Game/Combat/Player/Menu.Summon Menu` _output_get)
  ; Initialize the player and enemy health bars
  (`CombatPlayer.SetMovementAllowed` (`self.PlayerC`) false)
  (bind _returnvalue_2 (`|CreateWidget` "/Game/Combat/Player/HealthBarDisplay.HealthBarDisplay_C"))
  (bind _output_get_2 (set `self.healthBars` _returnvalue_2))
  (`UserWidget.AddToViewport` _output_get_2 0)
  (bind _returnvalue_3 (`CombatPlayer.GetHealth` (`self.PlayerC`)))
  (`/Game/Combat/Player/HealthBarDisplay.SetMaxHealthP` _healthbars _returnvalue_3)
  (bind _returnvalue_4 (`EnemyController.GetHealth` (`self.EnemyC`)))
  (`/Game/Combat/Player/HealthBarDisplay.SetMaxHealthE` _healthbars _returnvalue_4)
  (`self.Change Player Health`)
  (`self.Change Enemy Health`)
  (`/Game/Combat/Player/HealthBarDisplay.SetMenu` (`self.healthBars`) (`self.Menu`)))

(event `Reset Turn`
  (`/Game/Combat/Player/Menu.Summon Menu` (stale `self.ReceiveBeginPlay` _output_get))
  ; Update the health after each turn
  (`CombatPlayer.SetMovementAllowed` (`self.PlayerC`) false)
  (`self.Change Player Health`)
  (`self.Change Enemy Health`))

(event `Give Control to Enemy`
  (`WidgetBlueprintLibrary.SetInputMode_GameOnly` (`GameplayStatics.GetPlayerController` 0))
  (`/Game/Combat/Player/Menu.Unsummon Menu` (`self.Menu`))
  (`CombatPlayer.SetMovementAllowed` (`self.PlayerC`) true)
  (bind _returnvalue (`EnemyController.BeginEnemyAttack` (`self.EnemyC`)))
  (`KismetSystemLibrary.K2_SetTimerDelegate` (delegate `Reset Turn`) _returnvalue))

(fn `BeginTurn`
  (`/Game/Combat/Player/Menu.Summon Menu` (`self.Menu`)))

(fn `Change Enemy Health`
  (bind _returnvalue (`EnemyController.GetHealth` (`self.EnemyC`)))
  (`/Game/Combat/Player/HealthBarDisplay.UpdateEnemyHealth` (`self.healthBars`) _returnvalue))

(fn `Change Player Health`
  (bind _returnvalue (`CombatPlayer.GetHealth` (`self.PlayerC`)))
  (`/Game/Combat/Player/HealthBarDisplay.UpdatePlayerHealth` (`self.healthBars`) _returnvalue))

(fn `UserConstructionScript`)