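; Combat pawn Blueprint that handles the end of a fight by showing an end screen when the pawn or the enemy dies.
; OnPawnDeath and OnEnemyDeath each create their own end-screen widget, pause the game, switch to UI-only input focused on that widget and show the mouse cursor.
; BeginPlay, the IA_Move input event and the construction script are empty, so the graph holds no movement or combat logic.
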(event `self.ReceiveBeginPlay`)

(event `EnhancedInput|/Game/Inputs/IA_Move`
  (params (ActionValue :type "Vector2D Structure") (ElapsedSeconds :type "Float (double-precision)") (TriggeredSeconds :type "Float (double-precision)") (InputAction :type "InputAction Object Reference" :default "/Game/Inputs/IA_Move.IA_Move")))

(event `self.OnPawnDeath`
  (bind _returnvalue (`|CreateWidget` "/Game/Combat/Player/WBP_EndScreen01.WBP_EndScreen01_C"))
  (`UserWidget.AddToViewport` _returnvalue 0)
  (`GameplayStatics.SetGamePaused` true)
  (`WidgetBlueprintLibrary.SetInputMode_UIOnlyEx` (`GameplayStatics.GetPlayerController` 0) _returnvalue)
  (set `PlayerController.bShowMouseCursor` true (`GameplayStatics.GetPlayerController` 0)))

(event `self.OnEnemyDeath`
  (bind _returnvalue (`|CreateWidget` "/Game/Combat/Player/WBP_EndScreen02.WBP_EndScreen02_C"))
  (`UserWidget.AddToViewport` _returnvalue 0)
  (`GameplayStatics.SetGamePaused` true)
  (`WidgetBlueprintLibrary.SetInputMode_UIOnlyEx` (`GameplayStatics.GetPlayerController` 0) _returnvalue)
  (set `PlayerController.bShowMouseCursor` true (`GameplayStatics.GetPlayerController` 0)))

(fn `UserConstructionScript`)