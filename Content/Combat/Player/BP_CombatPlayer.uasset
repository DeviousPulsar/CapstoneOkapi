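; BP_CombatPlayer is the player's input layer for grid combat, covering attack, parry and movement.
; Left click passes LeftClickAttack to AttackGrid and right click calls Parry, while WASD sends unit direction vectors to Pawn.Move.
; Every input is gated by IsMovementAllowed, and the attack, parry and move logic is defined outside these graphs.
; A RightClickAttack reference sits unused in the event graph.
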(event `Key|LeftMouseButton`
  (params (Key :type "Key Structure"))
  ; Player Attack
  (:`Pressed`
    (if (`self.IsMovementAllowed`)
      (`self.AttackGrid` (`self.LeftClickAttack`)))))

(event `Key|RightMouseButton`
  (params (Key :type "Key Structure"))
  ; Player Attack
  (:`Pressed`
    (if (`self.IsMovementAllowed`)
      (`self.Parry`))))

(event `Key|W`
  (params (Key :type "Key Structure"))
  ; Player Movement
  (:`Pressed`
    (if (`self.IsMovementAllowed`)
      (`CombatPawn.Move` (`self.Pawn`) (0.0 -1.0)))))

(event `Key|S`
  (params (Key :type "Key Structure"))
  ; Player Movement
  (:`Pressed`
    (if (`self.IsMovementAllowed`)
      (`CombatPawn.Move` (`self.Pawn`) (0.0 1.0)))))

(event `Key|D`
  (params (Key :type "Key Structure"))
  ; Player Movement
  (:`Pressed`
    (if (`self.IsMovementAllowed`)
      (`CombatPawn.Move` (`self.Pawn`) (1.0 0.0)))))

(event `Key|A`
  (params (Key :type "Key Structure"))
  ; Player Movement
  (:`Pressed`
    (if (`self.IsMovementAllowed`)
      (`CombatPawn.Move` (`self.Pawn`) (-1.0 0.0)))))

(fn `UserConstructionScript`)